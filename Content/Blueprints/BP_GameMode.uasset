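; Game mode that spawns and possesses a BP_Player pawn for each player who logs in, on the authority only.
; PostLogin lazily caches all PlayerStarts, re-entering the check until the list is non-empty, then picks the one whose tag equals the running player count.
; Each successful spawn increments that count, with debug prints along the way.
; SpawnPlayers is empty, and its CreatePlayer-based batch spawn loop is disconnected.
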(event `self.K2_PostLogin`
  (params (NewPlayer :type "PlayerController Object Reference"))
  (`KismetSystemLibrary.PrintString` "OnPostLogin" true true (struct :`R` 1.0 :`A` 1.0) 5.0)
  (`/Engine/EditorBlueprintResources/ActorMacros.Switch Has Authority`
    (:`Authority`
      (if (> (`KismetArrayLibrary.Array_Length` (`self.player Spawn points`)) 0) :!label _label
        (`KismetSystemLibrary.PrintString` (`KismetStringLibrary.Concat_StrStr` "Current Player Count: " (`KismetStringLibrary.Conv_IntToString` (`self.playerCount`))) true true (struct :`G` 0.66 :`B` 1.0 :`A` 1.0) 5.0)
        (for _array_element (`self.player Spawn points`)
          (if (== (`PlayerStart.PlayerStartTag` _array_element) (`KismetStringLibrary.Conv_StringToName` (`KismetStringLibrary.Conv_IntToString` (`self.playerCount`))))
            (bind _returnvalue (`|SpawnActorFromClass` "/Game/Blueprints/BP_Player.BP_Player_C" (`self.GetTransform` _array_element) "AlwaysSpawn" "OverrideRootScale" null null))
            (`KismetSystemLibrary.PrintString` (`KismetStringLibrary.Concat_StrStr` "Player " (`KismetStringLibrary.Conv_IntToString` (`self.playerCount`)) " Spawned") true true (struct :`G` 0.66 :`B` 1.0 :`A` 1.0) 5.0)
            (`Controller.Possess` NewPlayer _returnvalue)
            (set `self.playerCount` (+ (`self.playerCount`) 1))
            (`KismetSystemLibrary.PrintString` (`KismetStringLibrary.Concat_StrStr` "Current Player Count: " (`KismetStringLibrary.Conv_IntToString` (`self.playerCount`))) true true (struct :`R` 1.0 :`A` 1.0) 5.0)
            (break)))
        (else
          (bind _outactors (`GameplayStatics.GetAllActorsOfClass` "/Script/Engine.PlayerStart"))
          (set `self.player Spawn points` _outactors)
          (goto _label))))))

(fn `GetPlayerStartPoint`
  (bind _outactors (`GameplayStatics.GetAllActorsOfClass` "/Script/Engine.PlayerStart"))
  (set `self.player Spawn points` _outactors))

(fn `SpawnPlayers`)

(fn `UserConstructionScript`)
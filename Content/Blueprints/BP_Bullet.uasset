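; BP_Bullet is a networked paintball-style projectile that damages players and leaves paint splats.
; On hit, the server damages a BP_Player and spawns the splat, while other hits spawn it without an authority check.
; Each decal gets a random size and a dynamic material with a random frame and the bullet's colour.
; The server destroys the bullet after impact or a five-second lifetime.
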(event `self.ReceiveHit`
  (params (MyComp :type "PrimitiveComponent Object Reference") (Other :type "Actor Object Reference") (OtherComp :type "PrimitiveComponent Object Reference") (bSelfMoved :type Boolean) (HitLocation :type "Vector Structure") (HitNormal :type "Vector Structure") (NormalImpulse :type "Vector Structure") (Hit :type "HitResult Structure (by ref)"))
  (bind _asbp_player (cast `/Game/Blueprints/BP_Player` Other)
    (:`then`
      (`/Engine/EditorBlueprintResources/ActorMacros.Switch Has Authority`
        (:`Authority`
          (`KismetSystemLibrary.PrintString` "Hit Player")
          (`/Game/Blueprints/BP_Player.Deal Damage` _asbp_player 10))))
    (:`CastFailed`
      _))
  ;[1 1 1] Spawn Painted Decal
  (bind _returnvalue (`GameplayStatics.SpawnDecalAtLocation` "/Game/Assets/Guns/Paint_Splat_M.Paint_Splat_M" (`KismetMathLibrary.Conv_DoubleToVector` (`KismetMathLibrary.RandomFloatInRange` 60.0 100.0)) HitLocation (`KismetMathLibrary.Conv_VectorToRotator` HitNormal)))
  (bind _returnvalue_2 (`DecalComponent.CreateDynamicMaterialInstance` _returnvalue))
  (`MaterialInstanceDynamic.SetScalarParameterValue` _returnvalue_2 "Frame" (`KismetMathLibrary.Conv_IntToDouble` (`KismetMathLibrary.RandomIntegerInRange` 0 3)))
  (`MaterialInstanceDynamic.SetVectorParameterValue` _returnvalue_2 "Colour" (`self.Color`))
  (`/Engine/EditorBlueprintResources/ActorMacros.Switch Has Authority` :!label _label
    (:`Authority`
      (`self.K2_DestroyActor`))))

(event `self.ReceiveBeginPlay`
  (`KismetSystemLibrary.Delay` 5.0)
  (goto _label))

(fn `UserConstructionScript`)